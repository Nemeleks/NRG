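; Player Blueprint with health and satiety components that puts a test widget on screen.
; On BeginPlay, only the non-authority branch creates WBP_TEST, stores it and adds it to the viewport, with no local-control check.
; An unconnected debug print of current HP and satiety remains in the graph, while Tick and the construction script do nothing.
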(event EventBeginPlay
  (Networking|SwitchHasAuthority
    (:Remote
      (bind _returnvalue (UserInterface|CreateWidget "/Game/UI/WBP_TEST.WBP_TEST_C"))
      (bind _output_get (Variables|Default|SetNewVar_0 _returnvalue))
      (UserInterface|Viewport|AddtoViewport _output_get 0))))

(event EventTick
  (params (DeltaSeconds :type Float%20%28single-precision%29)))

(fn ConstructionScript)